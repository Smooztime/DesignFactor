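; BP_PadChecker is a puzzle pad that detects whether a barrel on it has the same material as the pad.
; A looping timer box-traces for a BP_BaseBarrel, ignoring "Ground"-tagged actors, and switches both to MI_Atlas_01 on a match or restores their saved materials otherwise.
; End overlap restores matched materials and clears IsHit.
; Both paths update IsMatch and IsHit, then call OnSwitchMatchedColor.
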(event OnComponentEndOverlap(PadCollision)
  (params (OverlappedComponent :type Primitive%20Component%20Object%20Reference) (OtherActor :type Actor%20Object%20Reference) (OtherComp :type Primitive%20Component%20Object%20Reference) (OtherBodyIndex :type Integer))
  (bind _asbp_base_barrel (Utilities|Casting|CastToBP_BaseBarrel OtherActor))
  (CallFunction|SetMaterialBack _asbp_base_barrel _asbp_base_barrel _asbp_base_barrel))

(event Custom|CheckBarrelMat
  (CallFunction|CheckandSetMaterial))

(event EventBeginPlay
  (CallFunction|SetOldMaterial)
  (Utilities|Time|SetTimerbyEvent (delegate Custom|CheckBarrelMat) 0.1 true))

(fn ConstructionScript)

(fn CheckMat
  (params (MatObject :type BP%20Base%20Barrel%20Object%20Reference))
  (return (== (Rendering|Material|GetMaterial (Variables|/Game/Blueprints/Puzzle/Barrels/BP_BaseBarrel.BP_BaseBarrel_C|GetBarrel MatObject) 0) (Rendering|Material|GetMaterial (Variables|Default|GetPadChecker) 0))))

(fn VectorUp
  (return (+ (* (Math|Vector|GetUpVector (Variables|Default|GetPadChecker)) (Variables|Default|GetDistanceCheck)) (Variables|/Script/Engine.SceneComponent|GetRelativeLocation (Variables|Default|GetPadChecker)))))

(fn BoxTraceCheck
  (params (ActorsToIgnore :type Array%20of%20Actor%20Object%20References))
  (bind _outhit (Collision|BoxTraceByChannel (Variables|/Script/Engine.SceneComponent|GetRelativeLocation (Variables|Default|GetPadChecker)) (Math|Vector|GetUpVector (Variables|Default|GetPadChecker)) "100.000000,100.000000,20.000000" "0, 0, 0" "TraceTypeQuery1" false ActorsToIgnore "None" true "(R=1.000000,G=0.000000,B=0.000000,A=1.000000)" "(R=0.000000,G=1.000000,B=0.000000,A=1.000000)" 0.01))
  (return (.hitactor _outhit)))

(fn SetMaterialBack
  (params (MatObject :type BP%20Base%20Barrel%20Object%20Reference) (Target :type BP%20Base%20Barrel%20Object%20Reference) (Material :type BP%20Base%20Barrel%20Object%20Reference))
  (if (CallFunction|CheckMat MatObject)
    (Rendering|Material|SetMaterial (Variables|Default|GetPadChecker) 0 (Variables|Default|GetMatOld))
    (Rendering|Material|SetMaterial (Variables|/Game/Blueprints/Puzzle/Barrels/BP_BaseBarrel.BP_BaseBarrel_C|GetBarrel Target) 0 (Variables|/Game/Blueprints/Puzzle/Barrels/BP_BaseBarrel.BP_BaseBarrel_C|GetMatBarrelOld Material))
    (Variables|Default|SetbIsMatch true)
    (Variables|Default|SetbIsHit false)
    (Default|CallOnSwitchMatchedColor)
    (else
      (Variables|Default|SetbIsMatch false)
      (Variables|Default|SetbIsHit false)
      (Default|CallOnSwitchMatchedColor))))

(fn CheckandSetMaterial
  (bind _outactors (Actor|GetAllActorswithTag "Ground"))
  (bind _outhit_hitactor (CallFunction|BoxTraceCheck _outactors))
  (bind _asbp_base_barrel (Utilities|Casting|CastToBP_BaseBarrel _outhit_hitactor))
  (if (CallFunction|CheckMat _asbp_base_barrel)
    (Rendering|Material|SetMaterial (Variables|Default|GetPadChecker) 0 "/Game/Low_Poly_Viking_Interiors/Materials/Atlas/MI_Atlas_01.MI_Atlas_01")
    (Rendering|Material|SetMaterial (Variables|/Game/Blueprints/Puzzle/Barrels/BP_BaseBarrel.BP_BaseBarrel_C|GetBarrel _asbp_base_barrel) 0 "/Game/Low_Poly_Viking_Interiors/Materials/Atlas/MI_Atlas_01.MI_Atlas_01")
    (Variables|Default|SetbIsMatch true)
    (Variables|Default|SetbIsHit true)
    (Default|CallOnSwitchMatchedColor)
    (else
      (Rendering|Material|SetMaterial (Variables|Default|GetPadChecker) 0 (Variables|Default|GetMatOld))
      (Rendering|Material|SetMaterial (Variables|/Game/Blueprints/Puzzle/Barrels/BP_BaseBarrel.BP_BaseBarrel_C|GetBarrel _asbp_base_barrel) 0 (Variables|/Game/Blueprints/Puzzle/Barrels/BP_BaseBarrel.BP_BaseBarrel_C|GetMatBarrelOld _asbp_base_barrel))
      (Variables|Default|SetbIsMatch false)
      (Variables|Default|SetbIsHit true)
      (Default|CallOnSwitchMatchedColor))))

(fn SetOldMaterial
  (Variables|Default|SetMatOld (Rendering|Material|GetMaterial (Variables|Default|GetPadChecker) 0)))
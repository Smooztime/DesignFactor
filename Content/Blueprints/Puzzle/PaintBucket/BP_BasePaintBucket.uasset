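; Base paint bucket for a puzzle, which a character can carry and use to recolor barrels.
; Interaction events have the interacting character pick up the Bucket component and drop the held item when interaction stops.
; When BucketCollision overlaps a BP_BaseBarrel, it copies the Color component's first material onto the barrel mesh and saves it as that barrel's MatBarrelOld.
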(event OnComponentBeginOverlap(BucketCollision)
  (params (OverlappedComponent :type Primitive%20Component%20Object%20Reference) (OtherActor :type Actor%20Object%20Reference) (OtherComp :type Primitive%20Component%20Object%20Reference) (OtherBodyIndex :type Integer) (bFromSweep :type Boolean) (SweepResult :type Hit%20Result%20Structure%20%28by%20ref%29))
  (bind _color (Variables|Default|GetColor))
  (bind _returnvalue (Rendering|Material|GetMaterial _color 0))
  (bind _asbp_base_barrel (Utilities|Casting|CastToBP_BaseBarrel OtherActor))
  (Rendering|Material|SetMaterial (Variables|/Game/Blueprints/Puzzle/Barrels/BP_BaseBarrel.BP_BaseBarrel_C|GetBarrel _asbp_base_barrel) 0 _returnvalue)
  (Variables|/Game/Blueprints/Puzzle/Barrels/BP_BaseBarrel.BP_BaseBarrel_C|SetMatBarrelOld _asbp_base_barrel _returnvalue))

(event EventBeginInteractable
  (params (InteractingCharacter :type BP%20Base%20Character%20Object%20Reference))
  (Default|PickUpItem InteractingCharacter (Variables|Default|GetBucket)))

(event EventStopInteractable
  (params (InteractingCharacter :type BP%20Base%20Character%20Object%20Reference))
  (Default|DropItem InteractingCharacter))

(fn ConstructionScript)
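; Base character Blueprint providing Enhanced Input movement, jump, toggle crouch and sprint with a stamina UI.
; On possession it adds the character mapping context and creates the stamina widget.
; Sprint press and release switch walk speed and a state enum.
; Each press calls a one-shot stamina deduction that updates the widget only if IsSprint is true, a flag never set here; CanAct is an unused stub returning false.
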(event Input|EnhancedActionEvents|EnhancedInputActionIA_Movement
  (params (ActionValue :type Vector%202D%20Structure) (ElapsedSeconds :type Float%20%28double-precision%29) (TriggeredSeconds :type Float%20%28double-precision%29) (InputAction :type Input%20Action%20Object%20Reference :default "/Game/Blueprints/Input/Default/IA_Movement.IA_Movement"))
  (CallFunction|Movement ActionValue))

(event Input|EnhancedActionEvents|EnhancedInputActionIA_Sprint
  (params (ActionValue :type Boolean) (ElapsedSeconds :type Float%20%28double-precision%29) (TriggeredSeconds :type Float%20%28double-precision%29) (InputAction :type Input%20Action%20Object%20Reference :default "/Game/Blueprints/Input/Default/IA_Sprint.IA_Sprint"))
  (:Started
    (CallFunction|InitiateSprint))
  (:Completed
    (CallFunction|SolveSprint)))

(event Input|EnhancedActionEvents|EnhancedInputActionIA_Crouch
  (params (ActionValue :type Boolean) (ElapsedSeconds :type Float%20%28double-precision%29) (TriggeredSeconds :type Float%20%28double-precision%29) (InputAction :type Input%20Action%20Object%20Reference :default "/Game/Blueprints/Input/Default/IA_Crouch.IA_Crouch"))
  (:Started
    (Utilities|FlowControl|FlipFlop
      (:A
        (Character|Crouch))
      (:B
        (Character|UnCrouch)))))

(event Input|EnhancedActionEvents|EnhancedInputActionIA_Jump
  (params (ActionValue :type Boolean) (ElapsedSeconds :type Float%20%28double-precision%29) (TriggeredSeconds :type Float%20%28double-precision%29) (InputAction :type Input%20Action%20Object%20Reference :default "/Game/Blueprints/Input/Default/IA_Jump.IA_Jump"))
  (:Started
    (Character|Jump))
  (:Completed
    (Character|StopJumping)))

(event EventPossessed
  (params (NewController :type Controller%20Object%20Reference))
  (CallFunction|SetupInput)
  (bind _returnvalue (UserInterface|CreateWidget "/Game/Blueprints/UI/UI_Stamina.UI_Stamina_C"))
  (bind _output_get (Variables|Default|SetPlayerSP _returnvalue))
  (UserInterface|Viewport|AddtoViewport _output_get 0))

(fn ConstructionScript)

(fn SetupInput
  (bind _asplayer_controller (Utilities|Casting|CastToPlayerController (Pawn|GetController))
    (:then
      (Input|AddMappingContext (PlayerController|LocalPlayerSubsystems|GetEnhancedInputLocalPlayerSubsystem _asplayer_controller) "/Game/Blueprints/Input/Default/IMC_Character.IMC_Character" 0 "(bIgnoreAllPressedKeysUntilRelease=True,bForceImmediately=False,bNotifyUserSettings=False)"))
    (:CastFailed
      (Development|PrintString "Couldn't find player controller"))))

(fn CanAct
  (return false))

(fn Movement
  (params (AxisValue :type Vector%202D%20Structure))
  (Pawn|Input|AddMovementInput (Class|KismetMathLibrary|VectorRight) (.x AxisValue) false)
  (Pawn|Input|AddMovementInput (Class|KismetMathLibrary|VectorForward) (.y AxisValue) false))

(fn InitiateSprint
  (Variables|/Script/Engine.CharacterMovementComponent|SetMaxWalkSpeed (Variables|Character|GetCharacterMovement) 1e+03)
  (Variables|Default|SetCurrentState "NewEnumerator3")
  (CallFunction|UsedStamina))

(fn SolveSprint
  (Variables|/Script/Engine.CharacterMovementComponent|SetMaxWalkSpeed (Variables|Character|GetCharacterMovement) 6e+02)
  (Variables|Default|SetCurrentState "NewEnumerator1"))

(fn UsedStamina
  (if (Variables|Default|GetbIsSprint)
    (bind _output_get (Variables|Default|SetCurrentSP (- (Variables|Default|GetCurrentSP) 2.0)))
    (Default|SetStaminaPercentage (Variables|Default|GetPlayerSP) _output_get (Variables|Default|GetMaxSP))))